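; Child piece of a stacked obstacle that fades away and is destroyed once it lands on something else.
; A mesh hit that is not a sibling piece, stacked obstacle or projectile is treated as the floor, triggering Disappear once.
; Disappear removes the piece from its parent's child list, has the parent recheck its children, then drives a dynamic material's Opacity by timeline before destroying the actor.
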(event `self.StaticMesh.OnComponentHit`
  (params (HitComponent :type "PrimitiveComponent Object Reference") (OtherActor :type "Actor Object Reference") (OtherComp :type "PrimitiveComponent Object Reference") (NormalImpulse :type "Vector Structure") (Hit :type "HitResult Structure (by ref)"))
  (set `self.Other Actor` OtherActor)
  (cast `/Game/Blueprints/Obstacles/BP_ChildStackObstacle` (`self.Other Actor`)
    (:`CastFailed`
      (cast `/Game/Blueprints/Obstacles/BP_StackedObstacle` (`self.Other Actor`)
        (:`CastFailed`
          (cast `/Game/Blueprints/Projectiles/BP_BaseProjectile` (`self.Other Actor`)
            (:`CastFailed`
              (if (not (`self.HasHitFloor`))
                (`KismetSystemLibrary.PrintString` "HitFloor")
                (set `self.HasHitFloor` true)
                (`self.Event Disappear`)))))))))

(event `self.ReceiveBeginPlay`
  (bind _returnvalue (`PrimitiveComponent.CreateDynamicMaterialInstance` (`self.StaticMesh`) 0 (`PrimitiveComponent.GetMaterial` (`self.StaticMesh`) 0) "None"))
  (set `self.Dynamic Material` _returnvalue))

(event `Event Disappear`
  (`KismetArrayLibrary.Array_RemoveItem` (`/Game/Blueprints/Obstacles/BP_StackedObstacle.ChildObstacles` (`self.ParentObstacle`)) self)
  (`/Game/Blueprints/Obstacles/BP_StackedObstacle.Event CheckChildren` (`self.ParentObstacle`))
  (bind (_direction _opacity) (`Timeline|Timeline`)
    (:`Update`
      (`MaterialInstanceDynamic.SetScalarParameterValue` (`self.Dynamic Material`) "Opacity" _opacity))
    (:`Finished`
      (`self.K2_DestroyActor`))))

(fn `UserConstructionScript`)