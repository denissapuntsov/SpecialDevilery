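; Stacked obstacle that builds a column of child obstacles on its base and disappears once they are all gone.
; BeginPlay creates a dynamic material for the base, then spawns Height-driven children at scaled vertical offsets with random yaw, setting their parent reference and mass scale.
; CheckChildren tests for an empty child array and triggers a timeline that sets the base's opacity, then destroys the actor.
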(event `self.ReceiveBeginPlay`
  (bind _base (`self.Base`))
  (bind (_returnvalue_x _returnvalue_y _returnvalue_z) (`KismetMathLibrary.BreakVector` (`SceneComponent.K2_GetComponentScale` _base)))
  (bind (_returnvalue_x_2 _returnvalue_y_2 _returnvalue_z_2) (`KismetMathLibrary.BreakVector` (`SceneComponent.K2_GetComponentLocation` _base)))
  ; Assign Dynamic Material
  (bind _returnvalue (`PrimitiveComponent.CreateDynamicMaterialInstance` (`self.Base`) 0 (`PrimitiveComponent.GetMaterial` (`self.Base`) 0) "None"))
  (set `self.Dynamic Material` _returnvalue)
  ; Spawn Children
  (for _index (range (+ (`self.Height`) 1))
    (bind _returnvalue_2 (`|SpawnActorFromClass` "/Game/Blueprints/Obstacles/BP_ChildStackObstacle.BP_ChildStackObstacle_C" (`KismetMathLibrary.MakeTransform` (`KismetMathLibrary.MakeVector` _returnvalue_x_2 _returnvalue_y_2 (+ _returnvalue_z_2 (* (* (+ _index 1) 150.0) _returnvalue_z))) (`KismetMathLibrary.MakeRotator` 0.0 0.0 (`KismetMathLibrary.RandomFloatInRange` 10.0 200.0)) (`KismetMathLibrary.MakeVector` _returnvalue_x _returnvalue_y _returnvalue_z)) "Undefined" "MultiplyWithRoot" null null))
    (`KismetArrayLibrary.Array_Add` (`self.ChildObstacles`) _returnvalue_2)
    (set `/Game/Blueprints/Obstacles/BP_ChildStackObstacle.ParentObstacle` self _returnvalue_2)
    (`PrimitiveComponent.SetMassScale` (`/Game/Blueprints/Obstacles/BP_ChildStackObstacle.StaticMesh` _returnvalue_2) "None" (`self.MassScale`))))

(event `Event CheckChildren`
  ; If all children have been knocked over, fade the base out and destroy it
  (if (`KismetArrayLibrary.Array_IsEmpty` (`self.ChildObstacles`))
    (`self.EventDisappear`)))

(event `EventDisappear`
  ; Fade out
  (`Timeline|Timeline_0` :!via `PlayFromStart`
    (:`Update`
      (`MaterialInstanceDynamic.SetScalarParameterValue` (`self.Dynamic Material`) "Opacity" 0.0))
    (:`Finished`
      (`self.K2_DestroyActor`))))

(fn `UserConstructionScript`)