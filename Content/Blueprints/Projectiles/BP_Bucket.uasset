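; BP_Bucket is a scoring target that catches BP_BaseProjectile actors entering its Box trigger.
; On overlap it adds the projectile's DemonPoints through ScoreManager and destroys it, first posting a Wwise basket combo sound if ComboPoints meets a threshold.
; It then spawns an enlarged 3D onomatopoeia actor above the box and removes it after a short delay.
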(event `self.Box.OnComponentBeginOverlap`
  (params (OverlappedComponent :type "PrimitiveComponent Object Reference") (OtherActor :type "Actor Object Reference") (OtherComp :type "PrimitiveComponent Object Reference") (OtherBodyIndex :type Integer) (bFromSweep :type Boolean) (SweepResult :type "HitResult Structure (by ref)"))
  (bind (_returnvalue_x _returnvalue_y _returnvalue_z) (`KismetMathLibrary.BreakVector` (`SceneComponent.K2_GetComponentLocation` (`self.Box`))))
  (bind _asbp_base_projectile (cast `/Game/Blueprints/Projectiles/BP_BaseProjectile` OtherActor))
  (if (>= (`/Game/Blueprints/Projectiles/BP_BaseProjectile.Combo Points` _asbp_base_projectile) 5)
    (`AkGameplayStatics.PostEvent` "/Game/WwiseAudio/Events/Default_Work_Unit/SFX/LauncherComboBasket_Play.LauncherComboBasket_Play"))
  (`/Game/Blueprints/Managers/BP_ScoreManager.AddPoints` (`self.Score Manager`) (`/Game/Blueprints/Projectiles/BP_BaseProjectile.DemonPoints` _asbp_base_projectile))
  (`self.K2_DestroyActor` _asbp_base_projectile)
  (bind _returnvalue (`|SpawnActorFromClass` "/Game/Blueprints/Projectiles/BP_3D_Onomatopoeia.BP_3D_Onomatopoeia_C" (`KismetMathLibrary.MakeTransform` (`KismetMathLibrary.MakeVector` _returnvalue_x _returnvalue_y (+ _returnvalue_z 100.0)) (struct) (2.0 2.0 2.0)) "Undefined" "MultiplyWithRoot" null null))
  (`KismetSystemLibrary.Delay` 0.5)
  (`self.K2_DestroyActor` _returnvalue))

(fn `UserConstructionScript`)