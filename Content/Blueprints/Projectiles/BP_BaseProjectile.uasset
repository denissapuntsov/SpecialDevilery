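; Base projectile Blueprint that scores demon points on hits and switches to physics simulation on overlap.
; It finds the BP_LauncherManager on BeginPlay and asks it to unbind the projectile on any hit against an actor not tagged "NoHit".
; Such hits increment DemonPoints and, only if IsInvincible is already true, hold it briefly before clearing it.
; Box overlaps with anything other than projectiles or launchers enable physics.
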(event `self.ReceiveBeginPlay`
  ; Set Launcher Manager reference
  (bind _returnvalue (`GameplayStatics.GetActorOfClass` "/Game/Blueprints/Managers/BP_LauncherManager.BP_LauncherManager_C"))
  (set `self.Launcher Manager` _returnvalue))

(event `self.Projectile.OnComponentHit`
  (params (HitComponent :type "PrimitiveComponent Object Reference") (OtherActor :type "Actor Object Reference") (OtherComp :type "PrimitiveComponent Object Reference") (NormalImpulse :type "Vector Structure") (Hit :type "HitResult Structure (by ref)"))
  ; Process Hits
  ;; If hits anything but the bucket, add a point, remove 1 HP, give IFrames
  (if (not (`self.ActorHasTag` OtherActor "NoHit"))
    (`/Game/Blueprints/Managers/BP_LauncherManager.Event UnbindProjectile` (`self.Launcher Manager`) (`self.Projectile`))
    (set `self.DemonPoints` (+ 1 (`self.DemonPoints`)))
    (if (`self.IsInvincible`)
      (`|ExecutionSequence`
        (:`then_1`
          (set `self.IsInvincible` true)
          (`KismetSystemLibrary.Delay` 1.0)
          (set `self.IsInvincible` false))))))

(event `self.Box.OnComponentBeginOverlap`
  (params (OverlappedComponent :type "PrimitiveComponent Object Reference") (OtherActor :type "Actor Object Reference") (OtherComp :type "PrimitiveComponent Object Reference") (OtherBodyIndex :type Integer) (bFromSweep :type Boolean) (SweepResult :type "HitResult Structure (by ref)"))
  (cast `/Game/Blueprints/Projectiles/BP_BaseProjectile` OtherActor
    (:`CastFailed`
      (cast `/Game/Blueprints/Launchers/BP_Launcher` OtherActor
        (:`CastFailed`
          (`PrimitiveComponent.SetSimulatePhysics` (`self.Projectile`) true))))))

(fn `UserConstructionScript`)