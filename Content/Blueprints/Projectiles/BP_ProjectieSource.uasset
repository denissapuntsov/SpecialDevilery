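; Interactable projectile source that hands out a randomly chosen projectile to whoever interacts with it.
; ShuffleProjectile picks the next projectile at random from ProjectilePool, first on BeginPlay and again after each handout.
; On interact, it assigns the pre-picked projectile only if the instigator has no valid held projectile.
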(event `self.ReceiveBeginPlay`
  (`self.ShuffleProjectile`))

(event `/Game/FirstPerson/Blueprints/BPI_Interactable.OnInteract`
  (params (Instigator :type "/Game/FirstPerson/Blueprints/BP_FirstPersonCharacter Object Reference"))
  (`/Engine/EditorBlueprintResources/StandardMacros.IsValid` (`/Game/FirstPerson/Blueprints/BP_FirstPersonCharacter.HeldProjectile` Instigator)
    (:`Is Not Valid`
      (`/Game/FirstPerson/Blueprints/BP_FirstPersonCharacter.Assign New Projectile` Instigator (`self.NextProjectile`))
      (`self.ShuffleProjectile`))))

(fn `ShuffleProjectile`
  (set `self.NextProjectile` (`|GetArrayItem` (`self.ProjectilePool`) (`KismetMathLibrary.RandomInteger` (`KismetArrayLibrary.Array_Length` (`self.ProjectilePool`))))))

(fn `UserConstructionScript`)