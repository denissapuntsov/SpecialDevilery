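; Deprecated physics launcher that, when a BP_BaseProjectile hits its Collider, restarts that projectile's physics and applies an impulse intended to arc it to EndPoint.
; Hits are throttled by a short cooldown flag.
; LaunchProjectile stores direction, distance and a height difference taken from Y, then prints debug values.
; The angle-based ballistic math is disconnected, so BallisticImpulseVector is never computed here before use.
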(event `self.Collider.OnComponentHit`
  (params (HitComponent :type "PrimitiveComponent Object Reference") (OtherActor :type "Actor Object Reference") (OtherComp :type "PrimitiveComponent Object Reference") (NormalImpulse :type "Vector Structure") (Hit :type "HitResult Structure (by ref)"))
  ; Process Collision only once per 0.3 seconds
  (if (not (`self.IsHit`))
    (set `self.IsHit` true)
    (`|ExecutionSequence`
      (:`then_0`
        (bind _asbp_base_projectile (cast `/Game/Blueprints/Projectiles/BP_BaseProjectile` OtherActor))
        (set `self.Hit Location` Hit_Location)
        (`self.Launch Projectile` _asbp_base_projectile))
      (:`then_1`
        (`KismetSystemLibrary.Delay` 0.3)
        (set `self.IsHit` false)))))

(fn `Launch Projectile`
  (params (Projectile :type "/Game/Blueprints/Projectiles/BP_BaseProjectile Object Reference"))
  (bind (_direction_x _direction_y) (`KismetMathLibrary.BreakVector` (`self.Direction`)))
  (bind _interactingprojectile (`self.InteractingProjectile`))
  (set `self.InteractingProjectile` (`/Game/Blueprints/Projectiles/BP_BaseProjectile.Projectile` Projectile))
  (`|ExecutionSequence`
    (:`then_0`
      ; Get direction and distance
      (bind _output_get (set `self.Direction` (- (`SceneComponent.K2_GetComponentLocation` (`self.EndPoint`)) (`self.Hit Location`))))
      (set `self.Distance` (`KismetMathLibrary.VSize` _output_get))
      (set `self.Height Diff` _direction_y))
    (:`then_1`
      ; Reset Physics on interacting projectile
      (`PrimitiveComponent.SetSimulatePhysics` _interactingprojectile false))
    (:`then_2`
      (`PrimitiveComponent.SetSimulatePhysics` _interactingprojectile true))
    (:`then_3`
      ; Create a curve that reaches its peak at Zero Point and Terminates at End Point
      (`PrimitiveComponent.AddImpulse` (`self.InteractingProjectile`) (`self.Ballistic Impulse Vector`) "None" false)
      (`KismetSystemLibrary.PrintString` (`KismetStringLibrary.Conv_VectorToString` (`self.Hit Location`)))
      (`KismetSystemLibrary.PrintString` (`KismetStringLibrary.Conv_DoubleToString` (`self.Distance`))))))

(fn `UserConstructionScript`)