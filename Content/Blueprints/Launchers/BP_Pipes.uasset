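; BP_Pipes is a pipe teleporter that sucks in BP_BaseProjectile actors and sends them to another random pipe in the level.
; Trigger overlap applies an impulse oriented by the Entrance rotation, and a TeleportEntrance hit hides the projectile and pauses its physics.
; After a delay it reappears at a random pipe's Trigger, chosen from a list cached at BeginPlay.
; That pipe's suction is briefly disabled to avoid instant recapture.
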(event `self.ReceiveBeginPlay`
  ; Get reference to all other pipes in level
  (bind _outactors (`GameplayStatics.GetAllActorsOfClass` "BP_Pipes_C"))
  (bind _output_get (set `self.Pipes` _outactors))
  (`KismetArrayLibrary.Array_RemoveItem` _output_get self))

(event `self.Trigger.OnComponentBeginOverlap`
  (params (OverlappedComponent :type "PrimitiveComponent Object Reference") (OtherActor :type "Actor Object Reference") (OtherComp :type "PrimitiveComponent Object Reference") (OtherBodyIndex :type Integer) (bFromSweep :type Boolean) (SweepResult :type "HitResult Structure (by ref)"))
  (bind _asbp_base_projectile (cast `/Game/Blueprints/Projectiles/BP_BaseProjectile` OtherActor))
  (set `self.CurrentProjectile` (`/Game/Blueprints/Projectiles/BP_BaseProjectile.Projectile` _asbp_base_projectile))
  (if (`self.CanSuckItSillyStyle`)
    (`|ExecutionSequence`
      (:`then_0`
        ; Launch (suck in) projectile towards teleporter
        (`PrimitiveComponent.AddImpulse` (`self.CurrentProjectile`) (`KismetMathLibrary.GreaterGreater_VectorRotator` (0.0 0.0 1000.0) (`SceneComponent.K2_GetComponentRotation` (`self.Entrance`))) "None" true)))))

(event `self.Trigger.OnComponentEndOverlap`
  (params (OverlappedComponent :type "PrimitiveComponent Object Reference") (OtherActor :type "Actor Object Reference") (OtherComp :type "PrimitiveComponent Object Reference") (OtherBodyIndex :type Integer))
  (cast `/Game/Blueprints/Projectiles/BP_BaseProjectile` OtherActor))

(event `self.TeleportEntrance.OnComponentHit`
  (params (HitComponent :type "PrimitiveComponent Object Reference") (OtherActor :type "Actor Object Reference") (OtherComp :type "PrimitiveComponent Object Reference") (NormalImpulse :type "Vector Structure") (Hit :type "HitResult Structure (by ref)"))
  (cast `/Game/Blueprints/Projectiles/BP_BaseProjectile` OtherActor)
  (`PrimitiveComponent.SetSimulatePhysics` (`self.CurrentProjectile`) false)
  (`SceneComponent.SetVisibility` (`self.CurrentProjectile`) false true)
  (`KismetSystemLibrary.Delay` 2.0)
  (bind _output_get (set `self.Connected Pipe` (`KismetArrayLibrary.Array_Random` (`self.Pipes`))))
  (set `/Game/Blueprints/Launchers/BP_Pipes.CanSuckItSillyStyle` false _output_get)
  (`SceneComponent.K2_SetWorldLocation` (`self.CurrentProjectile`) (`SceneComponent.K2_GetComponentLocation` (`/Game/Blueprints/Launchers/BP_Pipes.Trigger` _output_get)) false true)
  (`PrimitiveComponent.SetSimulatePhysics` (`self.CurrentProjectile`) true)
  (`SceneComponent.SetVisibility` (`self.CurrentProjectile`) true true)
  (`KismetSystemLibrary.Delay` 1.0)
  (set `/Game/Blueprints/Launchers/BP_Pipes.CanSuckItSillyStyle` true (`self.Connected Pipe`)))

(fn `UserConstructionScript`)