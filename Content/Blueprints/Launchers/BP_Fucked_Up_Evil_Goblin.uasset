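; BP_Fucked_Up_Evil_Goblin is an actor that catches projectiles hitting its Plane and spits them back out.
; A caught BP_BaseProjectile is frozen and hidden, then after a delay is raised, revealed and given a fixed impulse.
; Plane collision is off during the cycle, and stays off if the hit actor fails the cast.
; BeginPlay picks a random BP_Launcher, but the selection is unused here.
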(event `self.ReceiveBeginPlay`
  (bind _outactors (`GameplayStatics.GetAllActorsOfClass` "/Game/Blueprints/Launchers/BP_Launcher.BP_Launcher_C"))
  (set `self.Launchers` _outactors)
  (`self.Select Random Launcher`))

(event `self.Plane.OnComponentHit`
  (params (HitComponent :type "PrimitiveComponent Object Reference") (OtherActor :type "Actor Object Reference") (OtherComp :type "PrimitiveComponent Object Reference") (NormalImpulse :type "Vector Structure") (Hit :type "HitResult Structure (by ref)"))
  (bind _caught_projectile (`self.Caught Projectile`))
  (bind _projectile (`/Game/Blueprints/Projectiles/BP_BaseProjectile.Projectile` _caught_projectile))
  (`/Engine/EditorBlueprintResources/StandardMacros.IsValid` (`self.Caught Projectile`)
    (:`Is Not Valid`
      (`PrimitiveComponent.SetCollisionEnabled` (`self.Plane`) "NoCollision")
      ; Hide the projectile
      (bind _asbp_base_projectile (cast `/Game/Blueprints/Projectiles/BP_BaseProjectile` OtherActor))
      (bind _output_get (set `self.Caught Projectile` _asbp_base_projectile))
      (bind _projectile_2 (`/Game/Blueprints/Projectiles/BP_BaseProjectile.Projectile` _output_get))
      (`PrimitiveComponent.SetSimulatePhysics` _projectile_2 false)
      (`SceneComponent.SetVisibility` _projectile_2 false true)
      (`KismetSystemLibrary.Delay` 2.0)
      (`self.K2_AddActorWorldOffset` _caught_projectile (0.0 0.0 100.0) false false)
      (`PrimitiveComponent.SetSimulatePhysics` _projectile true)
      (`PrimitiveComponent.AddImpulse` _projectile (50.0 50.0 0.0) "None" false)
      (`SceneComponent.SetVisibility` _projectile true true)
      (`KismetSystemLibrary.Delay` 1.0)
      (set `self.Caught Projectile` null)
      (`PrimitiveComponent.SetCollisionEnabled` (`self.Plane`) "QueryAndPhysics"))))

(fn `Select Random Launcher`
  (set `self.Selected Launcher` (`|GetArrayItem` (`self.Launchers`) (`KismetMathLibrary.RandomInteger` (`KismetArrayLibrary.Array_Length` (`self.Launchers`))))))

(fn `UserConstructionScript`)